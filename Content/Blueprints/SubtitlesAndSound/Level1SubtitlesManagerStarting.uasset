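; Level 1 subtitle manager actor that displays the opening narration script one line at a time.
; BeginPlay adds a SubsBP widget to the viewport, and ShowFirstLine or ShowLine call ShowNextLine with the Level1OpeningScript data table.
; ShowNextLine blanks the widget, waits briefly, then displays the row at CurrentRow and increments it, restarting at zero for a first line.
; ShowLine ignores its line and list inputs, always continuing the opening script.
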(event Custom|clearSubtitles
  (Default|DisplayLine (Variables|Default|GetSubtitlesWidgetRef)))

(event Custom|ShowNextLine
  (params (FirstLine :type Boolean) (NarrationList :type Data%20Table%20Object%20Reference))
  (Default|DisplayLine (Variables|Default|GetSubtitlesWidgetRef))
  (Utilities|FlowControl|Delay 0.1)
  (Variables|Default|SetCurrentNarrationList NarrationList)
  (if FirstLine
    (Variables|Default|SetCurrentRow 0)
    (bind _outrownames (DataTable|GetDataTableRowNames (Variables|Default|GetCurrentNarrationList)))
    (bind _returnvalue (Utilities|GetDataTableRow (Variables|Default|GetCurrentNarrationList) (Utilities|Array|Get(acopy) _outrownames (Variables|Default|GetCurrentRow)))
      (:then
        (Default|DisplayLine (Variables|Default|GetSubtitlesWidgetRef) (.LineToShow (Utilities|Struct|BreakSubtitlesStruct _returnvalue)))
        (bind _result (Math|Integer|IncrementInt (Variables|Default|GetCurrentRow))
          (:%20%20
            (Variables|Default|SetCurrentRow _result)))))
    (else
      (bind _outrownames_2 (DataTable|GetDataTableRowNames (Variables|Default|GetCurrentNarrationList)))
      (bind _returnvalue_2 (Utilities|GetDataTableRow (Variables|Default|GetCurrentNarrationList) (Utilities|Array|Get(acopy) _outrownames_2 (Variables|Default|GetCurrentRow)))
        (:then
          (Default|DisplayLine (Variables|Default|GetSubtitlesWidgetRef) (.LineToShow (Utilities|Struct|BreakSubtitlesStruct _returnvalue_2)))
          (bind _result_2 (Math|Integer|IncrementInt (Variables|Default|GetCurrentRow))
            (:%20%20
              (Variables|Default|SetCurrentRow _result_2))))))))

(event EventBeginPlay
  (bind _returnvalue (UserInterface|CreateWidget "/Game/Blueprints/SubtitlesAndSound/SubsBP.SubsBP_C"))
  (bind _output_get (Variables|Default|SetSubtitlesWidgetRef _returnvalue))
  (UserInterface|Viewport|AddtoViewport _output_get 0)
  (CallFunction|ClearSubtitles))

(fn ConstructionScript)

(fn ShowLine
  (params (FirstLine :type Boolean) (NarrationList :type Data%20Table%20Object%20Reference) (Target :type Self%20Object%20Reference))
  (CallFunction|ShowNextLine false "/Game/Blueprints/SubtitlesAndSound/Level1OpeningScript.Level1OpeningScript"))

(fn ShowFirstLine
  (params (Target :type Self%20Object%20Reference))
  (CallFunction|ShowNextLine true "/Game/Blueprints/SubtitlesAndSound/Level1OpeningScript.Level1OpeningScript"))

(fn ClearSubs
  (Default|DisplayLine (Variables|Default|GetSubtitlesWidgetRef)))