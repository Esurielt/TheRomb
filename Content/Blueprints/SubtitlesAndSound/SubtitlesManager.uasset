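; SubtitlesManager is an actor that shows narration subtitles one line at a time through a SubsBP widget.
; On BeginPlay it creates the widget, adds it to the viewport and blanks it.
; Each ShowNextLine call optionally switches the narration DataTable or restarts at its first row, displays the current row's LineToShow and advances the index.
; ClearSubtitles blanks the display, and debug strings report missing tables.
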(event Custom|ClearSubtitles
  (Default|DisplayLine (Variables|Default|GetSubtitlesWidgetRef)))

(event Custom|ShowNextLine
  (params (First :type Boolean) (Narration :type Data%20Table%20Object%20Reference))
  (Utilities|IsValid Narration
    (:Is%20Valid
      (Variables|Default|SetCurrentNarrationList Narration))
    (:Is%20Not%20Valid
      (Development|PrintString (Utilities|String|ToString(Integer) (Variables|Default|GetCurrentRow)))))
  (if First
    (Variables|Default|SetCurrentRow 0))
  (Utilities|IsValid (Variables|Default|GetCurrentNarrationList)
    (:Is%20Valid
      (bind _outrownames (DataTable|GetDataTableRowNames (Variables|Default|GetCurrentNarrationList)))
      (bind _returnvalue (Utilities|GetDataTableRow (Variables|Default|GetCurrentNarrationList) (Utilities|Array|Get(acopy) _outrownames (Variables|Default|GetCurrentRow)))
        (:then
          (Default|DisplayLine (Variables|Default|GetSubtitlesWidgetRef) (.LineToShow (Utilities|Struct|BreakSubtitlesStruct _returnvalue)))
          (Math|Integer|IncrementInt (Variables|Default|GetCurrentRow)))))
    (:Is%20Not%20Valid
      (Development|PrintString "DataTableNotValid"))))

(event EventBeginPlay
  (bind _returnvalue (UserInterface|CreateWidget "/Game/Blueprints/SubtitlesAndSound/SubsBP.SubsBP_C"))
  (bind _output_get (Variables|Default|SetSubtitlesWidgetRef _returnvalue))
  (UserInterface|Viewport|AddtoViewport _output_get 0)
  (CallFunction|ClearSubtitles))

(fn ConstructionScript)