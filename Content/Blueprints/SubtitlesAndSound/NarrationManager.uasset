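; NarrationManager holds Sequencer event endpoints that drive narration subtitles from sequence event tracks.
; Each event receives a bound SubtitlesManager and forwards straight to its ShowFirstLine, ShowLine or ClearSubs functions.
; The ShowLine variants differ in whether they pass the FirstLine flag, narration list and target through, leaving all display logic to SubtitlesManager.
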(event Custom|SubtitlesManager_Event_0
  (params (SubtitlesManager :type Subtitles%20Manager%20Object%20Reference))
  (Default|ShowLine SubtitlesManager false))

(event Custom|SubtitlesManager_Event_1
  (params (SubtitlesManager :type Subtitles%20Manager%20Object%20Reference) (FirstLine :type Boolean) (NarrationList :type Data%20Table%20Object%20Reference))
  (Default|ShowLine SubtitlesManager FirstLine NarrationList))

(event Custom|SubtitlesManager_Event_2
  (params (SubtitlesManager :type Subtitles%20Manager%20Object%20Reference) (Target :type %20Object%20Reference))
  (Default|ShowFirstLine SubtitlesManager Target))

(event Custom|SubtitlesManager_Event_3
  (params (SubtitlesManager :type Subtitles%20Manager%20Object%20Reference) (FirstLine :type Boolean) (NarrationList :type Data%20Table%20Object%20Reference) (Target :type %20Object%20Reference))
  (Default|ShowLine SubtitlesManager FirstLine NarrationList Target))

(event Custom|SubtitlesManager_Event_4
  (params (SubtitlesManager :type Subtitles%20Manager%20Object%20Reference) (FirstLine :type Boolean) (NarrationList :type Data%20Table%20Object%20Reference) (Target :type %20Object%20Reference))
  (Default|ShowLine SubtitlesManager FirstLine NarrationList Target))

(event Custom|SubtitlesManager_Event_5
  (params (SubtitlesManager :type Subtitles%20Manager%20Object%20Reference))
  (Default|ClearSubs SubtitlesManager))