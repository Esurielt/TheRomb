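; DeathFadeBlueprint is a trigger actor that fades in a full-screen widget, by its name a white screen, as the player nears its center.
; The widget is created invisible at BeginPlay, and Ph overlap events track whether the player pawn is inside.
; While inside, Tick sets opacity from squared distance to the Radius component, scaled to a 512-unit range.
; Leaving the Ph volume resets opacity to zero.
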(event OnComponentBeginOverlap(ph)
  (params (OverlappedComponent :type Primitive%20Component%20Object%20Reference) (OtherActor :type Actor%20Object%20Reference) (OtherComp :type Primitive%20Component%20Object%20Reference) (OtherBodyIndex :type Integer) (bFromSweep :type Boolean) (SweepResult :type Hit%20Result%20Structure%20%28by%20ref%29))
  (if (== OtherActor (Game|Player|GetPlayerPawn 0))
    (Variables|Default|Setinside true)))

(event OnComponentEndOverlap(ph)
  (params (OverlappedComponent :type Primitive%20Component%20Object%20Reference) (OtherActor :type Actor%20Object%20Reference) (OtherComp :type Primitive%20Component%20Object%20Reference) (OtherBodyIndex :type Integer))
  (if (== (Game|Player|GetPlayerPawn 0) OtherActor)
    (Variables|Default|Setinside false)
    (Widget|SetRenderOpacity (stale EventBeginPlay _returnvalue) 0.0)))

(event EventBeginPlay
  (bind _returnvalue (UserInterface|CreateWidget "/Game/Blueprints/WhiteScreen.WhiteScreen_C"))
  (Widget|SetRenderOpacity _returnvalue 0.0)
  (UserInterface|Viewport|AddtoViewport _returnvalue 0))

(event Collision|EventActorBeginOverlap
  (params (OtherActor :type Actor%20Object%20Reference)))

(event EventTick
  (params (DeltaSeconds :type Float%20%28single-precision%29))
  (if (Variables|Default|Getinside)
    (Widget|SetRenderOpacity (stale EventBeginPlay _returnvalue) (- 1.0 (/ (Class|KismetMathLibrary|VectorDistanceSquared (Transformation|GetWorldLocation (Variables|Default|GetRadius)) (Transformation|GetActorLocation (Game|Player|GetPlayerPawn 0))) 262144.0)))))

(fn ConstructionScript)