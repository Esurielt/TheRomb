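; Door actor that slides its cube mesh vertically, sinking when opened and rising when closed.
; Switch active and inactive events set the Opened flag.
; Tick moves a clamped Depth value at constant speed toward the lower or upper limit and applies it as the cube's relative Z location, without sweep.
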(event EventBeginPlay)

(event Collision|EventActorBeginOverlap
  (params (OtherActor :type Actor%20Object%20Reference)))

(event EventTick
  (params (DeltaSeconds :type Float%20%28single-precision%29))
  (bind _returnvalue (* DeltaSeconds 5e+02))
  (if (Variables|Default|Getopened)
    (Variables|Default|Setdepth (Math|Float|Max(Float) (- (Variables|Default|Getdepth) _returnvalue) -125.0))
    (else
      (Variables|Default|Setdepth (Math|Float|Min(Float) (+ (Variables|Default|Getdepth) _returnvalue) 125.0))))
  (Transformation|SetRelativeLocation (Variables|Default|GetCube) (Math|Vector|MakeVector 0.0 0.0 (Variables|Default|Getdepth)) false false))

(event EventSwitchActiveTick
  (Variables|Default|Setopened true))

(event EventSwitchInactiveTick
  (Variables|Default|Setopened false))

(fn ConstructionScript)