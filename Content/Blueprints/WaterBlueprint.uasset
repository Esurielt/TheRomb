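; Water volume actor that pushes the player upward while they are inside its box.
; Box begin and end overlap events set an Inside flag, only for player pawn 0.
; While the flag is set, Tick applies fluid friction through the character's CalcVelocity, then calls LaunchCharacter every frame, overriding vertical velocity with a small upward value and preserving horizontal motion.
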(event OnComponentBeginOverlap(Box)
  (params (OverlappedComponent :type Primitive%20Component%20Object%20Reference) (OtherActor :type Actor%20Object%20Reference) (OtherComp :type Primitive%20Component%20Object%20Reference) (OtherBodyIndex :type Integer) (bFromSweep :type Boolean) (SweepResult :type Hit%20Result%20Structure%20%28by%20ref%29))
  (if (== OtherActor (Game|Player|GetPlayerPawn 0))
    (Variables|Default|Setinside true)))

(event OnComponentEndOverlap(Box)
  (params (OverlappedComponent :type Primitive%20Component%20Object%20Reference) (OtherActor :type Actor%20Object%20Reference) (OtherComp :type Primitive%20Component%20Object%20Reference) (OtherBodyIndex :type Integer))
  (if (== OtherActor (Game|Player|GetPlayerPawn 0))
    (Variables|Default|Setinside false)))

(event EventBeginPlay)

(event Collision|EventActorBeginOverlap
  (params (OtherActor :type Actor%20Object%20Reference)))

(event EventTick
  (params (DeltaSeconds :type Float%20%28single-precision%29))
  (if (Variables|Default|Getinside)
    (bind _ascharacter (Utilities|Casting|CastToCharacter (Game|Player|GetPlayerPawn 0)))
    (Class|CharacterMovementComponent|CalcVelocity (Variables|/Script/Engine.Character|GetCharacterMovement _ascharacter) DeltaSeconds 2.0 true 0.0)
    (Character|LaunchCharacter _ascharacter "0, 0,50.000000" false true)))

(fn ConstructionScript)