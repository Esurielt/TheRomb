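; Floor switch actor that is pressed while a ThirdPersonCharacter or Box actor overlaps its trigger box.
; Each tick it rechecks the overlapping actors, then sends an active or inactive tick message to every linked ThingToActivate.
; The same state slides the Cube mesh down or back up at a constant, clamped speed to show the press.
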(event EventBeginPlay)

(event Collision|EventActorBeginOverlap
  (params (OtherActor :type Actor%20Object%20Reference)))

(event EventTick
  (params (DeltaSeconds :type Float%20%28single-precision%29))
  (bind _returnvalue (* DeltaSeconds 9e+01))
  (bind _thingtoactivate (Variables|Switch|GetthingToActivate))
  (Variables|Default|Setactivated false)
  (bind _array_element (Utilities|Array|ForEachLoopwithBreak (Collision|GetOverlappingActors (Variables|Default|GetBox) 0 :!class /Script/Engine.PrimitiveComponent) :!label _label)
    (:LoopBody
      (Utilities|Casting|CastToThirdPersonCharacter _array_element
        (:then
          _)
        (:CastFailed
          (Utilities|Casting|CastToBox _array_element)))
      (Variables|Default|Setactivated true)
      (goto _label Break))
    (:Completed
      (if (Variables|Default|Getactivated)
        (for _array_element_2 _thingtoactivate
          (Class|SwitchActivatableBlueprint|SwitchActiveTick(Message) _array_element_2))
        (Variables|Default|Setdepth (Math|Float|Max(Float) (- (Variables|Default|Getdepth) _returnvalue) -5.0))
        (else
          (for _array_element_3 _thingtoactivate
            (Class|SwitchActivatableBlueprint|SwitchInactiveTick(Message) _array_element_3))
          (Variables|Default|Setdepth (Math|Float|Min(Float) (+ (Variables|Default|Getdepth) _returnvalue) 1e+01))))
      (Transformation|SetRelativeLocation (Variables|Default|GetCube) (Math|Vector|MakeVector 0.0 0.0 (Variables|Default|Getdepth)) false false))))

(fn ConstructionScript)