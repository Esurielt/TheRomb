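; DeathBase is a death-causing hazard actor that kills whatever overlaps it and handles player respawn.
; On overlap it copies its RespawnPoint to RombGameInstance and destroys the actor and its attachments, flagging PlayerDeath and incrementing DeathCounter for ThirdPersonCharacters.
; A looping timer stands in for Tick, polling that flag to spawn and possess a new character at the stored point, then clearing it.
; The respawn sits behind a DoOnce with no reset.
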(event Custom|FakeEventTick
  (bind _asromb_game_instance (Utilities|Casting|CastToRombGameInstance (Game|GetGameInstance)))
  (if (Variables|/Game/GameSettings/RombGameInstance.RombGameInstance_C|GetPlayerDeath _asromb_game_instance)
    (Utilities|FlowControl|DoOnce false
      (:Completed
        (bind _returnvalue (Game|SpawnActorfromClass "/Game/Blueprints/ThirdPersonBP/Blueprints/ThirdPersonCharacter.ThirdPersonCharacter_C" (Math|Transform|MakeTransform (.location (Variables|/Game/GameSettings/RombGameInstance.RombGameInstance_C|GetRespawnPoint _asromb_game_instance)) "0, 0, 0" "1,1,1") "Undefined" 0 0))
        (Pawn|Possess (Game|GetPlayerController 0) _returnvalue)
        (Variables|/Game/GameSettings/RombGameInstance.RombGameInstance_C|SetPlayerDeath _asromb_game_instance false)))))

(event EventBeginPlay
  (Utilities|Time|SetTimerbyEvent (delegate Custom|FakeEventTick) 0.1 true))

(event Collision|EventActorBeginOverlap
  (params (OtherActor :type Actor%20Object%20Reference))
  (bind _asromb_game_instance (Utilities|Casting|CastToRombGameInstance (Game|GetGameInstance)))
  (Variables|/Game/GameSettings/RombGameInstance.RombGameInstance_C|SetRespawnPoint _asromb_game_instance (Variables|Default|GetRespawn%20point))
  (Actor|DestroyActor (Actor|GetAttachedActors OtherActor true))
  (Actor|DestroyActor OtherActor)
  (Utilities|Casting|CastToThirdPersonCharacter OtherActor)
  (bind _asromb_game_instance_2 (Utilities|Casting|CastToRombGameInstance (Game|GetGameInstance)))
  (Variables|/Game/GameSettings/RombGameInstance.RombGameInstance_C|SetPlayerDeath _asromb_game_instance_2 true)
  (Variables|/Game/GameSettings/RombGameInstance.RombGameInstance_C|SetDeath_Counter _asromb_game_instance_2 (+ (Variables|/Game/GameSettings/RombGameInstance.RombGameInstance_C|GetDeath_Counter _asromb_game_instance_2) 1)))

(fn ConstructionScript)